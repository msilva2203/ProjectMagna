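; Base character Blueprint that handles camera transitions and health feedback in response to character events.
; Camera and shoulder updates store new settings, then replay timelines with play rates derived from each transition time.
; Timeline updates lerp spring arm length, height and lateral socket offset toward those settings, negating the offset for the left shoulder.
; Health feedback scales post-process saturation by health percent; the action-state event is an empty stub.
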(event `self.OnActionStateChanged`
  (params (PreviousState :type "EActionState Enum" :default "None") (CurrentState :type "EActionState Enum" :default "None")))

(event `self.OnCameraSettingsUpdated`
  (params (NewCameraSettings :type "CameraSettings Structure"))
  (bind _output_get (set `self.CurrentCameraSettings` NewCameraSettings))
  (`TimelineComponent.SetPlayRate` (`self.TL_Camera`) (/ 1.0 (`.TransitionTime` (break `CameraSettings` _output_get))))
  (`TimelineComponent.PlayFromStart` (`self.TL_Camera`)))

(event `self.OnShoulderUpdated`
  (params (NewShoulder :type "EShoulder Enum" :default "Center") (NewShoulderSettings :type "ShoulderSettings Structure"))
  (bind _output_get (set `self.CurrentShoulderSettings` NewShoulderSettings))
  (`|ExecutionSequence`
    (:`then_0`
      (if (`|EnumEquality` NewShoulder "Left")
        (bind (_shoulderoffset _transitiontime) (break `ShoulderSettings` _output_get))
        (`|VariableSetRef` _shoulderoffset (* _shoulderoffset -1.0))))
    (:`then_1`
      (`TimelineComponent.SetPlayRate` (`self.TL_Shoulder`) (/ 1.0 _transitiontime))
      (`TimelineComponent.PlayFromStart` (`self.TL_Shoulder`)))))

(event `self.OnHealthFeedback`
  (params (NewHealth :type "Float (single-precision)") (NewMaxHealth :type "Float (single-precision)") (HealthPercent :type "Float (single-precision)"))
  (setmembers `PostProcessSettings` :`StructRef` (`CameraComponent.PostProcessSettings` (`self.CameraComponent`)) :`ColorSaturation` (`KismetMathLibrary.MakeVector4` HealthPercent HealthPercent HealthPercent HealthPercent)))

(fn `UpdateCamera`
  (params (Alpha :type "Float (double-precision)"))
  (bind _springarmcomponent (`self.SpringArmComponent`))
  (bind (_cameralength _cameraheight) (break `CameraSettings` (`self.CurrentCameraSettings`)))
  (set `SpringArmComponent.TargetArmLength` (`KismetMathLibrary.Lerp` (`SpringArmComponent.TargetArmLength` _springarmcomponent) _cameralength Alpha) (`self.SpringArmComponent`))
  (`SceneComponent.K2_SetRelativeLocation` (`self.SpringArmComponent`) (`KismetMathLibrary.MakeVector` 0.0 0.0 (`KismetMathLibrary.Lerp` (.z (`SceneComponent.RelativeLocation` _springarmcomponent)) _cameraheight Alpha)) false false))

(fn `UpdateShoulder`
  (params (Alpha :type "Float (double-precision)"))
  (set `SpringArmComponent.SocketOffset` (`KismetMathLibrary.MakeVector` 0.0 (`KismetMathLibrary.Lerp` (.y (`SpringArmComponent.SocketOffset` (`self.SpringArmComponent`))) (`.ShoulderOffset` (break `ShoulderSettings` (`self.CurrentShoulderSettings`))) Alpha)) (`self.SpringArmComponent`)))

(fn `UserConstructionScript`)